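; GA_Sprint is a GAS sprint ability that applies a speed GameplayEffect while the input is held.
; After an initial commit, it stores the effect handle and starts a looping timer that re-commits the ability every CostPeriodTime to charge the cost periodically.
; Input release or a failed re-commit removes the effect and clears the timer, ending the ability only if removal succeeds.
; A failed initial commit does not call EndAbility.
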(event `self.K2_ActivateAbility`
  (bind _returnvalue (`self.GetAbilitySystemComponentFromActorInfo`))
  (`KismetSystemLibrary.PrintString` "开始激活冲刺")
  (bind _returnvalue_2 (`self.K2_CommitAbility`))
  (if _returnvalue_2
    (`|ExecutionSequence`
      (:`then_0`
        (bind _output_get (set `self.SpecHandle` (`AbilitySystemComponent.MakeOutgoingSpec` _returnvalue (`self.SprintSpeedEffectClass`) 1.0 (`AbilitySystemComponent.MakeEffectContext` _returnvalue))))
        (bind _returnvalue_3 (`AbilitySystemComponent.BP_ApplyGameplayEffectSpecToSelf` (`self.GetAbilitySystemComponentFromActorInfo`) _output_get))
        (set `self.GamePlayEffect` _returnvalue_3))
      (:`then_1`
        (bind _returnvalue_4 (`KismetSystemLibrary.K2_SetTimerDelegate` (delegate `自定义事件`) (`self.CostPeriodTime`) true))
        (set `self.SprintCostTimer` _returnvalue_4))
      (:`then_2`
        (`AbilityTask_WaitInputRelease.WaitInputRelease` false
          (:`OnRelease`
            (bind _returnvalue_5 (`AbilitySystemComponent.RemoveActiveGameplayEffect` (`self.GetAbilitySystemComponentFromActorInfo`) (`self.GamePlayEffect`) -1 :!label _label))
            (`KismetSystemLibrary.K2_ClearAndInvalidateTimerHandle` (`self.SprintCostTimer`))
            (if _returnvalue_5
              (`self.K2_EndAbility`))))))))

(event `self.K2_OnEndAbility`
  (params (bWasCancelled :type Boolean)))

(event `自定义事件`
  (bind _returnvalue (`self.K2_CommitAbility`))
  (if (not _returnvalue)
    (goto _label)))